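; Test game mode for a turn-based grid tactics game that alternates joining players between two teams and runs their turns.
; Turns pass between TestPC controllers via a played list; once all have played, unit moved/acted flags reset and a new round starts.
; Movement checks range with Grid A*, draws the debug path, moves the unit and regenerates movement actors.
; The AI phase is only a flag, with no AI actions.
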(event Custom|StartMovement
  (bind _active_playercontrollerref (Variables|Default|GetActive%20PlayerControllerRef))
  (bind _active_playercontrollerref_2 (Variables|Default|GetActive%20PlayerControllerRef))
  (bind _activeunit (Variables|/Game/Blueprints/TestPC.TestPC_C|GetActiveUnit _active_playercontrollerref))
  (bind _destinationindex (Variables|/Game/Blueprints/TestPC.TestPC_C|GetDestinationIndex _active_playercontrollerref))
  (bind _activeunit_2 (Variables|/Game/Blueprints/TestPC.TestPC_C|GetActiveUnit _active_playercontrollerref_2))
  ;[1 1 1] MoveUnit
  (if (Variables|/Game/Blueprints/Unit_Base.Unit_Base_C|GetMovedThisTurn? (Variables|/Game/Blueprints/TestPC.TestPC_C|GetActiveUnit (Variables|Default|GetActive%20PlayerControllerRef)))
    (Development|PrintString "Already Moved")
    (else
      (bind (_found_path _isvalid) (Default|AStar (Variables|Default|GetGridRef) (Variables|/Game/Blueprints/GridANchor.GridAnchor_C|Getindex _activeunit) _destinationindex (Math|Conversions|ToFloat(Integer) (Variables|/Game/Blueprints/Unit_Base.Unit_Base_C|GetMovementRange _activeunit))))
      (if _isvalid
        (Utilities|FlowControl|Sequence
          (:then_0
            (for _array_element _found_path
              (Rendering|Debug|DrawDebugSphere (Default|IndextoLocation (Variables|Default|GetGridRef) _array_element true) 5e+01 12 "(R=1.000000,G=0.000000,B=0.000000,A=1.000000)" 2.0 5.0)))
          (:then_1
            (Default|MoveUnit (Variables|Default|GetGridRef) _activeunit_2 _destinationindex _found_path)
            (Default|GenerateMovementActors (Variables|Default|GetGridRef) (Variables|/Game/Blueprints/GridANchor.GridAnchor_C|Getindex _activeunit_2) (Variables|/Game/Blueprints/Unit_Base.Unit_Base_C|GetMovementRange _activeunit_2) (Variables|/Game/Blueprints/Unit_Base.Unit_Base_C|GetAttackRange _activeunit_2))))
        (else
          (Development|PrintString "YOU CANNOT REACH THIS"))))))

(event Custom|CheckTurn
  (for _array_element (CallFunction|GetUnitbyTeam (Variables|/Game/Blueprints/TestPC.TestPC_C|GetTeam (Variables|Default|GetActive%20PlayerControllerRef)))
    (if (Variables|/Game/Blueprints/Unit_Base.Unit_Base_C|GetMovedThisTurn? _array_element)
      _)))

(event Custom|EndPlayerTurn
  (params (Controller :type Controller%20Object%20Reference))
  ;[1 1 1] Ends The Turn for all player units---should add actions to this
  ;;[1 1 1] Add to "played" controllers and reset active, in attempt to find "next" player to play
  (Utilities|Array|AddUnique (Variables|Default|GetControllersPlayed) Controller)
  (Variables|Default|SetActive%20PlayerControllerRef 0)
  (bind _outactors (Actor|GetAllActorsOfClass "/Game/Blueprints/TestPC.TestPC_C"))
  (for _array_element _outactors
    (if (not (Utilities|Array|ContainsItem (Variables|Default|GetControllersPlayed) _array_element))
      ;;[1 1 1] pick next active controller for this turn
      (Variables|Default|SetActive%20PlayerControllerRef _array_element)))
  (Utilities|IsValid (Variables|Default|GetActive%20PlayerControllerRef)
    (:Is%20Valid
      (Default|BeginTurnServer (Variables|Default|GetActive%20PlayerControllerRef) (CallFunction|GetFirstAvailUnit (Variables|/Game/Blueprints/TestPC.TestPC_C|GetTeam (Variables|Default|GetActive%20PlayerControllerRef)))) ; Begin turn for the new player
    )
    (:Is%20Not%20Valid
      ;[1 1 1] All Players Have Played
      (if (Variables|Default|GetAiHasPlayed)
        ;;[1 1 1] if AI Played End Turn
        (CallFunction|EndRound)
        (else
          (Variables|Default|SetAiHasPlayed true)
          (CallFunction|EndRound))))))

(event Custom|Start%20Turn
  ;[1 1 1] Get all controllers, pick first one and begin turn for it
  (bind _output_get (Variables|Default|SetTurnCount (+ (stale _output_get) 1)))
  (bind _outactors (Actor|GetAllActorsOfClass "/Game/Blueprints/TestPC.TestPC_C"))
  (bind _output_get_2 (Variables|Default|SetActive%20PlayerControllerRef (Utilities|Array|Get(acopy) _outactors)))
  (Default|BeginTurnServer _output_get_2 (CallFunction|GetFirstAvailUnit (Variables|/Game/Blueprints/TestPC.TestPC_C|GetTeam _output_get_2))))

(event Custom|EndRound
  ;[1 1 1] Reset all units, clear played controllers, and start next Turn
  (Utilities|Array|Clear (Variables|Default|GetControllersPlayed))
  (bind _outactors (Actor|GetAllActorsOfClass "/Game/Blueprints/Unit_Base.Unit_Base_C"))
  (for _array_element _outactors
    (Variables|/Game/Blueprints/Unit_Base.Unit_Base_C|SetMovedThisTurn? _array_element false)
    (Variables|/Game/Blueprints/Unit_Base.Unit_Base_C|SetActedThisTurn? _array_element false))
  (Variables|Default|SetAiHasPlayed false)
  (CallFunction|StartTurn))

(event EventBeginPlay
  ;[1 1 1] Inisital Setup
  (Utilities|IsValid (Variables|Default|GetGridRef)
    (:Is%20Valid
      _)
    (:Is%20Not%20Valid
      (bind _outactors (Actor|GetAllActorsOfClass "/Game/Blueprints/Grid.Grid_C"))
      (bind _output_get (Variables|Default|SetGridRef (Utilities|Array|Get(acopy) _outactors)))))
  (Default|GatherUnits _output_get)
  (CallFunction|StartTurn))

(event EventTick
  (params (DeltaSeconds :type Float%20%28single-precision%29))
  ;[1 1 1] Inisital Setup
)

(event EventPostLogin
  (params (NewPlayer :type Player%20Controller%20Object%20Reference))
  ;[1 1 1] Set teams for player 1 and player 2
  (Utilities|FlowControl|Sequence
    (:then_0
      (bind _astest_pc (Utilities|Casting|CastToTestPC NewPlayer))
      (Utilities|FlowControl|FlipFlop
        (:A
          (Variables|/Game/Blueprints/TestPC.TestPC_C|SetTeam _astest_pc "NewEnumerator0"))
        (:B
          (Variables|/Game/Blueprints/TestPC.TestPC_C|SetTeam _astest_pc "NewEnumerator3"))))
    (:then_1
      (|CallParentFunction NewPlayer))))

(fn ConstructionScript)

(fn GetUnitbyTeam
  (params (Team :type Team%20Enum :default "NewEnumerator2"))
  (bind _outactors (Actor|GetAllActorsOfClass "/Game/Blueprints/Unit_Base.Unit_Base_C"))
  (for _array_element _outactors
    (if (Utilities|Enum|Equal(Enum) (Variables|/Game/Blueprints/Unit_Base.Unit_Base_C|GetTeam _array_element) Team)
      (Utilities|Array|AddUnique (LocalVariables|GetTeam%20Units) _array_element)))
  (return (LocalVariables|GetTeam%20Units)))

(fn GetFirstAvailUnit
  (params (Team :type Team%20Enum :default "NewEnumerator2"))
  (bind _array_element (Utilities|Array|ForEachLoopwithBreak (CallFunction|GetUnitbyTeam Team))
    (:LoopBody
      (if (not (Variables|/Game/Blueprints/Unit_Base.Unit_Base_C|GetMovedThisTurn? _array_element))
        (return _array_element)))))

(fn SpawnDefaultPawnfor
  (params (NewPlayer :type Controller%20Object%20Reference) (StartSpot :type Actor%20Object%20Reference))
  (bind _returnvalue (|CallParentFunction NewPlayer StartSpot))
  (bind _astest_pc (Utilities|Casting|CastToTestPC NewPlayer)
    (:then
      (Variables|/Game/Blueprints/TestPC.TestPC_C|SetActiveUnit _astest_pc (CallFunction|GetFirstAvailUnit (Variables|/Game/Blueprints/TestPC.TestPC_C|GetTeam _astest_pc))))
    (:CastFailed
      _))
  (return _returnvalue))