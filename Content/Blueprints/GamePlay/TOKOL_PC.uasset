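; Player controller for a networked, turn-based grid tactics game, handling camera panning, tile hover and click-driven unit orders.
; TestGM starts turns; server events handle selection, destinations, movement, attacks and turn end, while client events refresh range tiles and HUD.
; Clicks on the Grid resolve to tile indices to select, target or attack; clicking the shop calls the game mode.
; ActiveUnit's OnRep attaches the camera and rebinds move-finished.
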(event Custom|BeginTurn%20Client
  (bind _activeunit (Variables|Default|GetActiveUnit))
  ;[1 1 1] this is where youd wanna add anything like show hud, notify player its his turn etc.
  (Variables|Default|SetCurrentMouseSelectedUnit 0)
  (Default|ClearMovementActors (CallFunction|GetGrid))
  (CallFunction|ShowRangeTiles _activeunit (Variables|/Game/Blueprints/Units/Unit_Base.Unit_Base_C|GetMovedThisTurn? _activeunit) false)
  (Default|RefreshMainWidget (CallFunction|GetCastedHud)))

(event Custom|Unit%20FinishMove
  (CallFunction|ShowRangeTiles (Variables|Default|GetActiveUnit) false false)
  (CallFunction|SetDestinationIndexServer -1))

(event Custom|Cancel%20Attack
  (CallFunction|ShowRangeTiles (Variables|Default|GetActiveUnit) false false)
  (Variables|Default|SetBIsAttacking false)
  (Utilities|Array|Clear (Variables|Default|GetCurrentAttackTiles)))

(event Custom|EndGame
  (params (Won :type Boolean))
  (bind _returnvalue (UserInterface|CreateWidget "/Game/UI/EndGame.EndGame_C" 0 Won))
  (UserInterface|Viewport|AddtoViewport _returnvalue 0))

(event Custom|Set%20Destination%20Index%20Server
  (params (Destination :type Integer))
  ;[1 1 1] Ensure your selected destination index is replicated to server
  (bind _output_get (Variables|Default|SetDestinationIndex Destination)))

(event Custom|Select%20Unit%20Server
  (params (Unit :type Unit%20Base%20Object%20Reference))
  ;[1 1 1] Ensure Active Unit is replicated to Server (and subsequently to relevant player)
  (Variables|Default|SetActiveUnit Unit)
  (Variables|Default|SetDestinationIndex -1))

(event Custom|PerformAttack%20Server
  (params (Enemy :type Unit%20Base%20Object%20Reference))
  (bind _activeunit (Variables|Default|GetActiveUnit))
  (if (not (Variables|/Game/Blueprints/Units/Unit_Base.Unit_Base_C|GetActedThisTurn? _activeunit))
    (Game|Damage|ApplyDamage Enemy (Math|Conversions|ToFloat(Integer) (Variables|/Game/Blueprints/Units/Unit_Base.Unit_Base_C|GetAttack _activeunit)) self (Variables|Default|GetActiveUnit))
    (Variables|/Game/Blueprints/Units/Unit_Base.Unit_Base_C|SetActedThisTurn? (Variables|Default|GetActiveUnit) true)))

(event Custom|Move%20Unit%20Server
  ;[1 1 1] Ensure Movement is executed on server
  (Default|StartMovement (Variables|Default|GetGameModeRef)))

(event Custom|End%20Turn%20Client
  (Default|ClearMovementActors (CallFunction|GetGrid))
  (Default|RefreshWidget (Variables|/Game/Blueprints/GamePlay/IngameHUD.IngameHUD_C|GetMainHUD_Ref (CallFunction|GetCastedHud))))

(event Custom|BeginTurn%20Server
  (params (ActiveUnit :type Unit%20Base%20Object%20Reference))
  (bind _team (Variables|Default|GetTeam))
  (bind _gamemoderef (Variables|Default|GetGameModeRef))
  (bind _unit (Default|GetFirstAvailUnit _gamemoderef _team))
  ;[1 1 1] Gamemode triggered, notifies this controller of being "active"
  (Utilities|IsValid (stale _output_get)
    (:Is%20Valid
      (bind _output_get (Variables|Default|SetActiveUnit ActiveUnit))
      (Variables|Default|SetisActive true :!label _label)
      (CallFunction|BeginTurnClient))
    (:Is%20Not%20Valid
      (Utilities|IsValid _unit
        (:Is%20Valid
          (Variables|Default|SetActiveUnit _unit)
          (goto _label))
        (:Is%20Not%20Valid
          (CallFunction|EndTurnServer))))))

(event Custom|BeginAttack
  (bind _attacktiles (CallFunction|ShowRangeTiles (Variables|Default|GetActiveUnit) true false))
  (Variables|Default|SetCurrentAttackTiles _attacktiles)
  (Variables|Default|SetBIsAttacking true))

(event Custom|End%20Turn%20Server
  ;[1 1 1] Notify Gamemode of ending turn
  (Variables|Default|SetisActive false)
  (CallFunction|EndTurnClient)
  (Default|EndPlayerTurn (Variables|Default|GetGameModeRef) self)
  (Development|PrintString "End Turn"))

(event EventBeginPlay
  (Variables|Default|SetbShowMouseCursor true)
  (Utilities|FlowControl|Sequence
    (:then_0
      (bind _astest_gm (Utilities|Casting|CastToTestGM (Game|GetGameMode)))
      (Variables|Default|SetGameModeRef _astest_gm))
    (:then_1
      (Default|RefreshMainWidget (CallFunction|GetCastedHud)))))

(event Input|AxisEvents|InputAxisMoveForward
  (params (AxisValue :type Float%20%28single-precision%29))
  ;[1 1 1] Camera Mov
  (Transformation|AddActorWorldOffset (Pawn|GetControlledPawn) (* (Transformation|GetActorForwardVector (Pawn|GetControlledPawn)) (|((Axis*DeltaSec)*MovementSpeed) AxisValue (Utilities|Time|GetWorldDeltaSeconds) 4e+02))))

(event Input|AxisEvents|InputAxisMouseMove
  (params (AxisValue :type Float%20%28single-precision%29))
  (bind _destinationindex (Variables|Default|GetDestinationIndex))
  (if (Variables|Default|GetisActive)
    (bind _posindex (CallFunction|SetMarkeronGrid))
    (Default|MoveMarker (CallFunction|GetMarker) (select (!= _destinationindex -1) _destinationindex _posindex))
    (bind _output_get (Variables|Default|SetCurrentMouseSelectedUnit (.Unit (Default|HasUnit (CallFunction|GetGrid) _posindex))))
    (Default|RefreshHoveredUnitInfo (CallFunction|GetCastedHud) _output_get)))

(event Input|AxisEvents|InputAxisMoveRight
  (params (AxisValue :type Float%20%28single-precision%29))
  ;[1 1 1] Camera Mov
  (Transformation|AddActorWorldOffset (Pawn|GetControlledPawn) (* (Transformation|GetActorRightVector (Pawn|GetControlledPawn)) (|((Axis*DeltaSec)*MovementSpeed) AxisValue (Utilities|Time|GetWorldDeltaSeconds) 4e+02))))

(event Input|MouseEvents|LeftMouseButton
  (params (Key :type Key%20Structure :default "None"))
  (:Pressed
    (if (Variables|Default|GetisActive)
      (CallFunction|OnClick))))

(fn ConstructionScript)

(fn OnClick
  (bind _hitresult (Game|Player|GetHitResultUnderCursorbyChannel "TraceTypeQuery1" true))
  (bind (_bblockinghit _binitialoverlap _time _distance _location _impactpoint _normal _impactnormal _physmat _hitactor) (Collision|BreakHitResult _hitresult))
  (Variables|Default|SetCurrentMouseSelectedUnit 0)
  (Utilities|FlowControl|Sequence
    (:then_0
      (if _bblockinghit
        (Variables|Default|SetRelativeLocation (- _location (Transformation|GetActorLocation _hitactor)))
        (if (not (== (Utilities|GetClass _hitactor) "/Game/Blueprints/Units/Unit_Base.Unit_Base_C"))
          (if (== (Utilities|GetClass _hitactor) "/Game/Blueprints/Grid/Grid.Grid_C")
            (if (Utilities|Enum|Equal(Enum) (Variables|/Game/Blueprints/Units/Unit_Base.Unit_Base_C|GetTeam (Variables|Default|GetActiveUnit)) (Variables|Default|GetTeam))
              (bind _asgrid (Utilities|Casting|CastToGrid _hitactor))
              (if (.hasUnit (Default|HasUnit (CallFunction|GetGrid) (Default|VectortoIndex _asgrid (Variables|Default|GetRelativeLocation))))
                (if (Utilities|Enum|Equal(Enum) (Variables|/Game/Blueprints/Units/Unit_Base.Unit_Base_C|GetTeam (.Unit (Default|HasUnit (CallFunction|GetGrid) (Default|VectortoIndex _asgrid (Variables|Default|GetRelativeLocation))))) (Variables|Default|GetTeam))
                  (CallFunction|SelectUnitServer (.Unit (Default|HasUnit (CallFunction|GetGrid) (Default|VectortoIndex _asgrid (Variables|Default|GetRelativeLocation)))))
                  (CallFunction|ShowRangeTiles (.Unit (Default|HasUnit (CallFunction|GetGrid) (Default|VectortoIndex _asgrid (Variables|Default|GetRelativeLocation)))) false false)
                  (elif (Variables|Default|GetBIsAttacking)
                    (CallFunction|PerformAttackServer (.Unit (Default|HasUnit (CallFunction|GetGrid) (Default|VectortoIndex _asgrid (Variables|Default|GetRelativeLocation)))))
                    (CallFunction|ShowRangeTiles (Variables|Default|GetActiveUnit) false false)))
                (else
                  (CallFunction|SetDestinationIndexServer (Default|VectortoIndex _asgrid (Variables|Default|GetRelativeLocation)))))
              (else
                (Development|PrintString "you do not have a player unit selected")))
            (elif (== (Utilities|GetClass _hitactor) "/Game/Blueprints/Grid/Shop_BP.Shop_BP_C")
              (Default|SetupShop (Variables|Default|GetGameModeRef) (Default|IndextoLocation (Variables|Default|GetGridRef) 113 true))
              (else
                (Development|PrintString "Did not select a grid")))))))
    (:then_1
      (Variables|Default|SetBIsAttacking false))))

(fn SetMarkeronGrid
  (bind _hmm (Variables|Default|Gethmm))
  (bind (_hitresult _returnvalue) (Class|PlayerController|GetHitResultUnderCursorforObjects _hmm true))
  (bind (_bblockinghit _binitialoverlap _time _distance _location _impactpoint _normal _impactnormal _physmat _hitactor) (Collision|BreakHitResult _hitresult))
  (if _returnvalue
    (Utilities|IsValid (CallFunction|GetGrid)
      (:Is%20Valid
        (Variables|Default|SetRelativeLocation (- _location (Transformation|GetActorLocation _hitactor)))
        (return (Default|VectortoIndex (CallFunction|GetGrid) (Variables|Default|GetRelativeLocation)))))))

(fn GetMarker
  (Utilities|IsValid (Variables|Default|GetMarker)
    (:Is%20Valid
      _)
    (:Is%20Not%20Valid
      (bind _returnvalue (Game|SpawnActorfromClass "/Game/Blueprints/Grid/MarkerBP.MarkerBP_C" (Math|Transform|MakeTransform "0, 0, 0" "0, 0, 0" "1,1,1") "Undefined" 0 0))
      (bind _output_get (Variables|Default|SetMarker _returnvalue))))
  (return _output_get))

(fn OnRepActiveUnit
  (bind _returnvalue (Pawn|GetControlledPawn))
  (bind _activeunit (Variables|Default|GetActiveUnit))
  ;[1 1 1] this is when we receive "replicated" value for Active Unit, ensure camera goes to it
  (Utilities|FlowControl|Sequence
    (:then_0
      (Utilities|IsValid (Variables|Default|GetOld_ActiveUnit)
        (:Is%20Valid
          (EventDispatchers|UnbindallEventsfromMoveFinished (Variables|Default|GetOld_ActiveUnit)))))
    (:then_1
      (Variables|Default|SetOld_ActiveUnit _activeunit)
      (Utilities|IsValid _activeunit
        (:Is%20Valid
          (EventDispatchers|BindEventtoMoveFinished _activeunit (EventDispatchers|CreateEvent :!event Custom|Unit%20FinishMove))
          (if (.bSuccess (Utilities|Casting|CastToDefaultCamera (Pawn|GetControlledPawn)))
            (Transformation|AttachActorToActor _returnvalue _activeunit "None" "SnapToTarget" "KeepWorld" "SnapToTarget" true)
            (Transformation|SetActorRelativeTransform _returnvalue (Math|Transform|MakeTransform "0, 0,800.000000" "0, 0, 0" "1,1,1") false false)))))
    (:then_2
      (Default|RefreshUnitInfo (CallFunction|GetCastedHud)))))

(fn GetGrid
  (Utilities|IsValid (Variables|Default|GetGridRef)
    (:Is%20Valid
      (return (Variables|Default|GetGridRef)))
    (:Is%20Not%20Valid
      (bind _outactors (Actor|GetAllActorsOfClass "/Game/Blueprints/Grid/Grid.Grid_C"))
      (if (Utilities|Array|IsValidIndex _outactors)
        (bind _output_get (Variables|Default|SetGridRef (Utilities|Array|Get(acopy) _outactors)))
        (return _output_get)
        (else
          (return 0))))))

(fn ShowRangeTiles
  (params (Unit :type Unit%20Base%20Object%20Reference) (AttackOnly :type Boolean) (NoVisual :type Boolean))
  (bind (_walktiles _attacktiles_outer _all_attack_tiles) (Default|GenerateMovementActors (CallFunction|GetGrid) (Variables|/Game/Blueprints/Grid/GridAnchor.GridAnchor_C|Getindex Unit) (select (or (Variables|/Game/Blueprints/Units/Unit_Base.Unit_Base_C|GetMovedThisTurn? Unit) AttackOnly) 0 (Variables|/Game/Blueprints/Units/Unit_Base.Unit_Base_C|GetMovementRange Unit)) (Math|Float|SelectFloat 0.0 (Variables|/Game/Blueprints/Units/Unit_Base.Unit_Base_C|GetAttackRange Unit) (Variables|/Game/Blueprints/Units/Unit_Base.Unit_Base_C|GetActedThisTurn? Unit)) (Variables|/Game/Blueprints/Units/Unit_Base.Unit_Base_C|GetMinAttackRange Unit) (Variables|/Game/Blueprints/Units/Unit_Base.Unit_Base_C|GetSurface%20Cost%20Map Unit) false))
  (return _walktiles _attacktiles_outer _all_attack_tiles))

(fn GetCastedHud
  (bind _returnvalue (HUD|GetHUD))
  (if (== (Variables|Default|GetHUD_ref) _returnvalue)
    (return (Variables|Default|GetHUD_ref))
    (else
      (bind _asingame_hud (Utilities|Casting|CastToIngameHUD _returnvalue))
      (bind _output_get (Variables|Default|SetHUD_ref _asingame_hud))
      (return _output_get))))