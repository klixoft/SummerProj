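; Game mode for a turn-based grid tactics game, running rounds between player teams and a spawned AI controller.
; Logins alternate between two teams; each controller plays in turn, then the AI, before all units reset for the next round.
; Movement requests run grid A* within the active unit's range, draw debug spheres and move it.
; Teams without available units leave the grid's active list, ending the game when one or none remain.
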(event Custom|Endgame
  (bind _outactors (Actor|GetAllActorsOfClass "/Game/Blueprints/GamePlay/TestPC.TestPC_C"))
  (for _array_element _outactors
    (Default|EndGame _array_element (Utilities|Array|ContainsItem (Variables|/Game/Blueprints/Grid/Grid.Grid_C|GetActiveTeams (Variables|Default|GetGridRef)) (Variables|/Game/Blueprints/GamePlay/TestPC.TestPC_C|GetTeam _array_element)))))

(event Custom|StartMovement
  (bind _unit (CallFunction|GetActiveUnit))
  (bind _unit_2 (CallFunction|GetActiveUnit))
  (bind _active_playercontrollerref (Variables|Default|GetActive%20PlayerControllerRef))
  (bind _aiturn (Variables|Default|GetAiTurn))
  (bind _aicontroller (Variables|Default|GetAiController))
  (bind _destinationindex (Variables|/Game/Blueprints/GamePlay/TestPC.TestPC_C|GetDestinationIndex _active_playercontrollerref))
  (bind _destinationindex_2 (Variables|/Game/Blueprints/GamePlay/BasicAI.BasicAI_C|GetDestinationIndex _aicontroller))
  (bind _returnvalue (select _aiturn _destinationindex_2 _destinationindex))
  ;[1 1 1] MoveUnit
  (if (Variables|/Game/Blueprints/Units/Unit_Base.Unit_Base_C|GetMovedThisTurn? (CallFunction|GetActiveUnit))
    (Development|PrintString "Already Moved")
    (else
      (bind (_found_path _isvalid) (Default|AStar (Variables|Default|GetGridRef) (Variables|/Game/Blueprints/Grid/GridAnchor.GridAnchor_C|Getindex _unit_2) _returnvalue (Math|Conversions|ToFloat(Integer) (Variables|/Game/Blueprints/Units/Unit_Base.Unit_Base_C|GetMovementRange _unit_2)) (Variables|/Game/Blueprints/Units/Unit_Base.Unit_Base_C|GetSurface%20Cost%20Map _unit_2) false))
      (if _isvalid
        (Utilities|FlowControl|Sequence
          (:then_0
            (for _array_element _found_path
              (Rendering|Debug|DrawDebugSphere (Default|IndextoLocation (Variables|Default|GetGridRef) _array_element true) 5e+01 12 "(R=1.000000,G=0.000000,B=0.000000,A=1.000000)" 2.0 5.0)))
          (:then_1
            (Default|MoveUnit (Variables|Default|GetGridRef) _unit _returnvalue _found_path)
            (Default|GenerateMovementActors (Variables|Default|GetGridRef) (Variables|/Game/Blueprints/Grid/GridAnchor.GridAnchor_C|Getindex _unit) (Variables|/Game/Blueprints/Units/Unit_Base.Unit_Base_C|GetMovementRange _unit) (Variables|/Game/Blueprints/Units/Unit_Base.Unit_Base_C|GetAttackRange _unit) (Variables|/Game/Blueprints/Units/Unit_Base.Unit_Base_C|GetMinAttackRange _unit) (Variables|/Game/Blueprints/Units/Unit_Base.Unit_Base_C|GetSurface%20Cost%20Map _unit) false)))
        (else
          (Development|PrintString "YOU CANNOT REACH THIS"))))))

(event Custom|EndPlayerTurn
  (params (Controller :type Controller%20Object%20Reference))
  (bind _aicontroller (Variables|Default|GetAiController))
  (bind _team (Variables|/Game/Blueprints/GamePlay/BasicAI.BasicAI_C|GetTeam _aicontroller))
  (bind _unit (CallFunction|GetFirstAvailUnit _team))
  ;[1 1 1] Ends The Turn for all player units---should add actions to this
  ;;[1 1 1] Add to "played" controllers and reset active, in attempt to find "next" player to play
  (Utilities|Array|AddUnique (Variables|Default|GetControllersPlayed) Controller)
  (Variables|Default|SetActive%20PlayerControllerRef 0)
  (bind _outactors (Actor|GetAllActorsOfClass "/Game/Blueprints/GamePlay/TestPC.TestPC_C"))
  (for _array_element _outactors
    (if (not (Utilities|Array|ContainsItem (Variables|Default|GetControllersPlayed) _array_element))
      ;;[1 1 1] pick next active controller for this turn
      (Variables|Default|SetActive%20PlayerControllerRef _array_element)))
  (Utilities|IsValid (Variables|Default|GetActive%20PlayerControllerRef)
    (:Is%20Valid
      (Utilities|IsValid (CallFunction|GetFirstAvailUnit (Variables|/Game/Blueprints/GamePlay/TestPC.TestPC_C|GetTeam (Variables|Default|GetActive%20PlayerControllerRef)))
        (:Is%20Valid
          (Default|BeginTurnServer (Variables|Default|GetActive%20PlayerControllerRef) (CallFunction|GetFirstAvailUnit (Variables|/Game/Blueprints/GamePlay/TestPC.TestPC_C|GetTeam (Variables|Default|GetActive%20PlayerControllerRef)))) ; Begin turn for the new player
        )
        (:Is%20Not%20Valid
          (CallFunction|EndgameforTeam (Variables|/Game/Blueprints/GamePlay/TestPC.TestPC_C|GetTeam (Variables|Default|GetActive%20PlayerControllerRef))))))
    (:Is%20Not%20Valid
      ;[1 1 1] All Players Have Played
      (if (Variables|Default|GetAiHasPlayed)
        ;;[1 1 1] if AI Played End Turn
        (CallFunction|EndRound)
        (else
          (Utilities|IsValid _unit
            (:Is%20Valid
              (Variables|Default|SetAiTurn true)
              (Default|BeginTurnServer (Variables|Default|GetAiController) _unit))
            (:Is%20Not%20Valid
              (CallFunction|EndgameforTeam _team))))))))

(event Custom|Start%20Turn
  ;[1 1 1] Get all controllers, pick first one and begin turn for it
  (bind _output_get (Variables|Default|SetTurnCount (+ (stale _output_get) 1)))
  (bind _array_element (CallFunction|PickPlayer :!label _label))
  (Utilities|IsValid _array_element
    (:Is%20Valid
      (bind _output_get_2 (Variables|Default|SetActive%20PlayerControllerRef _array_element))
      (Utilities|IsValid (CallFunction|GetFirstAvailUnit (Variables|/Game/Blueprints/GamePlay/TestPC.TestPC_C|GetTeam _output_get_2))
        (:Is%20Valid
          (Default|BeginTurnServer _output_get_2 (CallFunction|GetFirstAvailUnit (Variables|/Game/Blueprints/GamePlay/TestPC.TestPC_C|GetTeam _output_get_2))))
        (:Is%20Not%20Valid
          (Utilities|Array|Add (Variables|Default|GetControllersEnded) (Variables|Default|GetActive%20PlayerControllerRef))
          (CallFunction|EndgameforTeam (Variables|/Game/Blueprints/GamePlay/TestPC.TestPC_C|GetTeam _output_get_2))
          (goto _label))))
    (:Is%20Not%20Valid
      (CallFunction|Endgame))))

(event Custom|EndRound
  ;[1 1 1] Reset all units, clear played controllers, and start next Turn
  (Utilities|Array|Clear (Variables|Default|GetControllersPlayed))
  (bind _outactors (Actor|GetAllActorsOfClass "/Game/Blueprints/Units/Unit_Base.Unit_Base_C"))
  (for _array_element _outactors
    (Variables|/Game/Blueprints/Units/Unit_Base.Unit_Base_C|SetMovedThisTurn? _array_element false)
    (Variables|/Game/Blueprints/Units/Unit_Base.Unit_Base_C|SetActedThisTurn? _array_element false))
  (Variables|Default|SetAiHasPlayed false)
  (Variables|Default|SetAiTurn false)
  (CallFunction|StartTurn))

(event Custom|SetupShop
  (params (SpawnPoint :type Vector))
  (bind _returnvalue (UserInterface|CreateWidget "/Game/UI/Shop/Shop.Shop_C" (Game|GetPlayerController 0) 0 SpawnPoint))
  (bind _output_get (Variables|Default|SetShopRef _returnvalue))
  (UserInterface|Viewport|AddtoViewport _output_get 0))

(event EventBeginPlay
  ;[1 1 1] Inisital Setup
  (Utilities|IsValid (Variables|Default|GetGridRef)
    (:Is%20Valid
      _)
    (:Is%20Not%20Valid
      (bind _outactors (Actor|GetAllActorsOfClass "/Game/Blueprints/Grid/Grid.Grid_C"))
      (bind _output_get (Variables|Default|SetGridRef (Utilities|Array|Get(acopy) _outactors)))))
  (Default|GatherUnits _output_get)
  (bind _returnvalue (Game|SpawnActorfromClass "/Game/Blueprints/GamePlay/BasicAI.BasicAI_C" (Math|Transform|MakeTransform "0, 0, 0" "0, 0, 0" "1,1,1") "Undefined" 0 0))
  (Variables|Default|SetAiController _returnvalue)
  (CallFunction|StartTurn))

(event EventTick
  (params (DeltaSeconds :type Float%20%28single-precision%29))
  ;[1 1 1] Inisital Setup
)

(event EventPostLogin
  (params (NewPlayer :type Player%20Controller%20Object%20Reference))
  ;[1 1 1] Set teams for player 1 and player 2
  (Utilities|FlowControl|Sequence
    (:then_0
      (bind _astest_pc (Utilities|Casting|CastToTestPC NewPlayer))
      (Utilities|FlowControl|FlipFlop
        (:A
          (Variables|/Game/Blueprints/GamePlay/TestPC.TestPC_C|SetTeam _astest_pc "NewEnumerator0"))
        (:B
          (Variables|/Game/Blueprints/GamePlay/TestPC.TestPC_C|SetTeam _astest_pc "NewEnumerator3"))))
    (:then_1
      (|CallParentFunction NewPlayer))))

(fn ConstructionScript)

(fn GetUnitbyTeam
  (params (Team :type Team%20Enum :default "NewEnumerator2"))
  (bind _outactors (Actor|GetAllActorsOfClass "/Game/Blueprints/Units/Unit_Base.Unit_Base_C"))
  (for _array_element _outactors
    (if (Utilities|Enum|Equal(Enum) (Variables|/Game/Blueprints/Units/Unit_Base.Unit_Base_C|GetTeam _array_element) Team)
      (Utilities|Array|AddUnique (LocalVariables|GetTeam%20Units) _array_element)))
  (return (LocalVariables|GetTeam%20Units)))

(fn GetFirstAvailUnit
  (params (Team :type Team%20Enum :default "NewEnumerator2"))
  (bind _array_element (Utilities|Array|ForEachLoopwithBreak (CallFunction|GetUnitbyTeam Team))
    (:LoopBody
      (if (not (Variables|/Game/Blueprints/Units/Unit_Base.Unit_Base_C|GetMovedThisTurn? _array_element))
        (return _array_element)))))

(fn SpawnDefaultPawnfor
  (params (NewPlayer :type Controller%20Object%20Reference) (StartSpot :type Actor%20Object%20Reference))
  (bind _returnvalue (|CallParentFunction NewPlayer StartSpot))
  (bind _astest_pc (Utilities|Casting|CastToTestPC NewPlayer)
    (:then
      (Variables|/Game/Blueprints/GamePlay/TestPC.TestPC_C|SetActiveUnit _astest_pc (CallFunction|GetFirstAvailUnit (Variables|/Game/Blueprints/GamePlay/TestPC.TestPC_C|GetTeam _astest_pc))))
    (:CastFailed
      _))
  (return _returnvalue))

(fn EndgameforTeam
  (params (Team :type Team%20Enum :default "NewEnumerator2"))
  (bind _gridref (Variables|Default|GetGridRef))
  (bind _activeteams (Variables|/Game/Blueprints/Grid/Grid.Grid_C|GetActiveTeams _gridref))
  (Utilities|Array|RemoveItem _activeteams Team)
  (if (<= (Utilities|Array|Length _activeteams) 1)
    (CallFunction|Endgame)
    (else
      (CallFunction|EndRound))))

(fn GetActiveUnit
  (return (select (Variables|Default|GetAiTurn) (Variables|/Game/Blueprints/GamePlay/BasicAI.BasicAI_C|GetActiveUnit (Variables|Default|GetAiController)) (Variables|/Game/Blueprints/GamePlay/TestPC.TestPC_C|GetActiveUnit (Variables|Default|GetActive%20PlayerControllerRef)))))

(fn PickPlayer
  (bind _outactors (Actor|GetAllActorsOfClass "/Game/Blueprints/GamePlay/TestPC.TestPC_C"))
  (bind _array_element (Utilities|Array|ForEachLoopwithBreak _outactors)
    (:LoopBody
      (if (not (Utilities|Array|ContainsItem (Variables|Default|GetControllersEnded) _array_element))
        (return _array_element)))
    (:Completed
      (return 0))))