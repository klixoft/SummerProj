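; In-game HUD Blueprint that owns the MainHud widget and relays refresh requests to it for the main view, unit info and hovered unit.
; InitWidget creates the widget, adds it to the viewport and caches the reference, running on BeginPlay.
; Each refresh event checks that reference and lazily initializes the widget when it is missing, so refresh requests do not rely on BeginPlay having run.
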(event Custom|Refresh_MainWidget
  (bind _mainhud_ref (Variables|Default|GetMainHUD_Ref))
  (Utilities|IsValid _mainhud_ref
    (:Is%20Valid
      (Default|RefreshWidget _mainhud_ref))
    (:Is%20Not%20Valid
      (CallFunction|InitWidget)
      (CallFunction|RefreshMainWidget))))

(event Custom|Refresh_HoveredUnitInfo
  (params (Unit :type Unit%20Base%20Object%20Reference))
  (Utilities|IsValid (Variables|Default|GetMainHUD_Ref)
    (:Is%20Valid
      _)
    (:Is%20Not%20Valid
      (CallFunction|InitWidget)
      (CallFunction|RefreshMainWidget)))
  (Default|RefreshHoveredUnit (Variables|Default|GetMainHUD_Ref) Unit))

(event Custom|Refresh_UnitInfo
  (Utilities|IsValid (Variables|Default|GetMainHUD_Ref)
    (:Is%20Valid
      _)
    (:Is%20Not%20Valid
      (CallFunction|InitWidget)
      (CallFunction|RefreshMainWidget)))
  (Default|RefreshUnitInfo (Variables|Default|GetMainHUD_Ref)))

(event EventBeginPlay
  (CallFunction|InitWidget)
  (CallFunction|RefreshMainWidget))

(fn ConstructionScript)

(fn InitWidget
  (Utilities|IsValid (Variables|Default|GetMainHUD_Ref)
    (:Is%20Not%20Valid
      (bind _returnvalue (UserInterface|CreateWidget "/Game/UI/MainHud.MainHud_C"))
      (UserInterface|Viewport|AddtoViewport _returnvalue 100)
      (Variables|Default|SetMainHUD_Ref _returnvalue))))