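; AI controller for a turn-based grid tactics game that plays its team's units, then notifies TestGM the turn is over.
; BrainTick attacks an enemy already in range, and if the unit hasn't moved, seeks one within move-plus-attack range.
; It intersects tiles that can hit that target with walkable tiles and moves along the cheapest A* path.
; Move-finished callbacks, bound in OnRep_ActiveUnit, re-run BrainTick or select the next available unit.
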(event Custom|BeginTurn%20AI%20Clients
  (bind _activeunit (Variables|Default|GetActiveUnit))
  ;[1 1 1] this is where youd wanna add anything like show hud, notify player its his turn etc.
  (Variables|Default|SetCurrentSelectedEnemyUnit 0)
  (Default|ClearMovementActors (CallFunction|GetGrid))
  (CallFunction|ShowRangeTiles _activeunit (Variables|/Game/Blueprints/Units/Unit_Base.Unit_Base_C|GetMovedThisTurn? _activeunit) false))

(event Custom|Unit%20FinishMove
  (CallFunction|ShowRangeTiles (Variables|Default|GetActiveUnit) false false)
  (CallFunction|SetDestinationIndexServer -1)
  (if (Variables|/Game/Blueprints/Units/Unit_Base.Unit_Base_C|GetActedThisTurn? (Variables|Default|GetActiveUnit))
    (CallFunction|SelectNextUnit)
    (else
      (CallFunction|BrainTick))))

(event Custom|Set%20Destination%20Index%20Server
  (params (Destination :type Integer))
  ;[1 1 1] Ensure your selected destination index is replicated to server
  (Variables|Default|SetDestinationIndex Destination))

(event Custom|Select%20Unit%20Server
  (params (Unit :type Unit%20Base%20Object%20Reference))
  ;[1 1 1] Ensure Active Unit is replicated to Server (and subsequently to relevant player)
  (Variables|Default|SetActiveUnit Unit)
  (Variables|Default|SetDestinationIndex -1))

(event Custom|PerformAttack%20Server
  (params (Enemy :type Unit%20Base%20Object%20Reference))
  (Game|Damage|ApplyDamage Enemy (Math|Conversions|ToFloat(Integer) (Variables|/Game/Blueprints/Units/Unit_Base.Unit_Base_C|GetAttack (Variables|Default|GetActiveUnit))) self (Variables|Default|GetActiveUnit))
  (if (Variables|/Game/Blueprints/Units/Unit_Base.Unit_Base_C|GetMovedThisTurn? (Variables|Default|GetActiveUnit))
    (Utilities|FlowControl|Delay 0.5)
    (CallFunction|SelectNextUnit)))

(event Custom|Move%20Unit%20Server
  ;[1 1 1] Ensure Movement is executed on server
  (Default|StartMovement (Variables|Default|GetGameModeRef)))

(event Custom|BeginTurn%20Server
  (params (ActiveUnit :type Unit%20Base%20Object%20Reference))
  ;[1 1 1] Gamemode triggered, notifies this controller of being "active"
  (Variables|Default|SetActiveUnit ActiveUnit)
  (Variables|Default|SetisActive true)
  (CallFunction|BeginTurnAIClients)
  (CallFunction|BrainTick))

(event Custom|BeginAttack
  (params (Enemy :type Unit%20Base%20Object%20Reference))
  (CallFunction|ShowRangeTiles (Variables|Default|GetActiveUnit) true false)
  (Variables|/Game/Blueprints/Units/Unit_Base.Unit_Base_C|SetActedThisTurn? (Variables|Default|GetActiveUnit) true)
  (Utilities|FlowControl|Delay 1.0)
  (CallFunction|PerformAttackServer Enemy))

(event Custom|End%20Turn%20Server
  (bind _gamemoderef (Variables|Default|GetGameModeRef))
  ;[1 1 1] Notify Gamemode of ending turn
  (Variables|Default|SetisActive false)
  (Default|ClearMovementActors (CallFunction|GetGrid))
  (Variables|/Game/Blueprints/GamePlay/TestGM.TestGM_C|SetAiTurn _gamemoderef false)
  (Variables|/Game/Blueprints/GamePlay/TestGM.TestGM_C|SetAiHasPlayed _gamemoderef true)
  (Default|EndPlayerTurn _gamemoderef self))

(event EventBeginPlay
  (bind _astest_gm (Utilities|Casting|CastToTestGM (Game|GetGameMode)))
  (Variables|Default|SetGameModeRef _astest_gm))

(fn ConstructionScript)

(fn OnRepActiveUnit
  (bind _activeunit (Variables|Default|GetActiveUnit))
  ;[1 1 1] this is when we receive "replicated" value for Active Unit, ensure camera goes to it
  (Utilities|FlowControl|Sequence
    (:then_0
      (Utilities|IsValid (Variables|Default|GetOld_ActiveUnit)
        (:Is%20Valid
          (EventDispatchers|UnbindallEventsfromMoveFinished (Variables|Default|GetOld_ActiveUnit)))))
    (:then_1
      (Variables|Default|SetOld_ActiveUnit _activeunit)
      (Utilities|IsValid _activeunit
        (:Is%20Valid
          (EventDispatchers|BindEventtoMoveFinished _activeunit (EventDispatchers|CreateEvent :!event Custom|Unit%20FinishMove)))))))

(fn GetGrid
  (Utilities|IsValid (Variables|Default|GetGridRef)
    (:Is%20Valid
      (return (Variables|Default|GetGridRef)))
    (:Is%20Not%20Valid
      (bind _outactors (Actor|GetAllActorsOfClass "/Game/Blueprints/Grid/Grid.Grid_C"))
      (if (Utilities|Array|IsValidIndex _outactors)
        (bind _output_get (Variables|Default|SetGridRef (Utilities|Array|Get(acopy) _outactors)))
        (return _output_get)
        (else
          (return 0))))))

(fn ShowRangeTiles
  (params (Unit :type Unit%20Base%20Object%20Reference) (AttackOnly :type Boolean) (NoVisual :type Boolean))
  (bind (_walktiles _attacktiles_outer _all_attack_tiles) (Default|GenerateMovementActors (CallFunction|GetGrid) (Variables|/Game/Blueprints/Grid/GridAnchor.GridAnchor_C|Getindex Unit) (select (or (Variables|/Game/Blueprints/Units/Unit_Base.Unit_Base_C|GetMovedThisTurn? Unit) AttackOnly) 0 (Variables|/Game/Blueprints/Units/Unit_Base.Unit_Base_C|GetMovementRange Unit)) (Math|Float|SelectFloat 0.0 (Variables|/Game/Blueprints/Units/Unit_Base.Unit_Base_C|GetAttackRange Unit) (Variables|/Game/Blueprints/Units/Unit_Base.Unit_Base_C|GetActedThisTurn? Unit)) (Variables|/Game/Blueprints/Units/Unit_Base.Unit_Base_C|GetMinAttackRange Unit) (Variables|/Game/Blueprints/Units/Unit_Base.Unit_Base_C|GetSurface%20Cost%20Map Unit) false))
  (return _walktiles _attacktiles_outer _all_attack_tiles))

(fn BrainTick
  (bind _activeunit (Variables|Default|GetActiveUnit))
  (bind _activeunit_2 (Variables|Default|GetActiveUnit))
  (Utilities|FlowControl|Sequence
    (:then_0
      (if (not (Variables|/Game/Blueprints/Units/Unit_Base.Unit_Base_C|GetActedThisTurn? _activeunit_2)) ; did we perform an action?
        ;[1 1 1] Find enemies with Attack Range (stationary)
        (bind _attacktiles_outer (CallFunction|ShowRangeTiles _activeunit_2 true true))
        (bind _array_element (Utilities|Array|ForEachLoopwithBreak _attacktiles_outer :!label _label)
          (:LoopBody
            (if (.hasUnit (Default|HasUnit (CallFunction|GetGrid) _array_element))
              (if (Utilities|Enum|NotEqual(Enum) (Variables|/Game/Blueprints/Units/Unit_Base.Unit_Base_C|GetTeam (.Unit (Default|HasUnit (CallFunction|GetGrid) _array_element))) (Variables|Default|GetTeam))
                (Utilities|FlowControl|Sequence
                  (:then_0
                    (goto _label Break))
                  (:then_1
                    (CallFunction|BeginAttack (.Unit (Default|HasUnit (CallFunction|GetGrid) _array_element)))))))))))
    (:then_1
      (if (Variables|/Game/Blueprints/Units/Unit_Base.Unit_Base_C|GetMovedThisTurn? _activeunit) ; have we moved this turn?
        (CallFunction|SelectNextUnit)
        (return)
        (else
          ;[1 1 1] Find enemies walk range (even if we need to move)
          (bind (_walktiles _attacktiles_outer_2 _attackablefromcurrentpos) (CallFunction|ShowRangeTiles _activeunit false false))
          (LocalVariables|SetWalkableTiles _walktiles)
          (bind _array_element_2 (Utilities|Array|ForEachLoopwithBreak _attackablefromcurrentpos :!label _label_2)
            (:LoopBody
              (if (.hasUnit (Default|HasUnit (CallFunction|GetGrid) _array_element_2))
                (if (Utilities|Enum|NotEqual(Enum) (Variables|/Game/Blueprints/Units/Unit_Base.Unit_Base_C|GetTeam (.Unit (Default|HasUnit (CallFunction|GetGrid) _array_element_2))) (Variables|Default|GetTeam))
                  (Utilities|FlowControl|Sequence
                    (:then_0
                      (Variables|/Game/Blueprints/Units/Unit_Base.Unit_Base_C|SetMovedThisTurn? (Variables|Default|GetActiveUnit) true)
                      (goto _label_2 Break))
                    (:then_1
                      (Variables|Default|SetCurrentSelectedEnemyUnit (.Unit (Default|HasUnit (CallFunction|GetGrid) _array_element_2)))
                      ;[1 1 1] Find all tiles we can attack this target from, and pick the "best" one
                      (bind _attacktiles (CallFunction|FindAttackTiles (Variables|Default|GetCurrentSelectedEnemyUnit) (LocalVariables|GetWalkableTiles)))
                      (LocalVariables|SetTempAttackTiles _attacktiles)
                      (for _array_element_3 (LocalVariables|GetTempAttackTiles)
                        (bind (_found_path _isvalid _pathcost) (Default|AStar (CallFunction|GetGrid) (Variables|/Game/Blueprints/Grid/GridAnchor.GridAnchor_C|Getindex (Variables|Default|GetActiveUnit)) _array_element_3 999.0 (Variables|/Game/Blueprints/Units/Unit_Base.Unit_Base_C|GetSurface%20Cost%20Map (Variables|Default|GetActiveUnit)) true))
                        (if (<= _pathcost (LocalVariables|GetTempCost))
                          (LocalVariables|SetTempCost _pathcost)
                          (LocalVariables|SetTempPath _found_path)))
                      (if (!= (LocalVariables|GetTempCost) 9999.0) ; did we find a path?
                        (Default|MoveUnit (CallFunction|GetGrid) (Variables|Default|GetActiveUnit) (Utilities|Array|Get(acopy) (LocalVariables|GetTempPath)) (LocalVariables|GetTempPath))))))))
            (:Completed
              ;[1 1 1] End turn for this unit if no enemies in range
              (if (not (Variables|/Game/Blueprints/Units/Unit_Base.Unit_Base_C|GetMovedThisTurn? (Variables|Default|GetActiveUnit)))
                (Variables|/Game/Blueprints/Units/Unit_Base.Unit_Base_C|SetMovedThisTurn? (Variables|Default|GetActiveUnit) true)
                (CallFunction|SelectNextUnit)))))))))

(fn SelectNextUnit
  (bind _gamemoderef (Variables|Default|GetGameModeRef))
  (bind _unit (Default|GetFirstAvailUnit _gamemoderef "NewEnumerator1"))
  (Utilities|IsValid _unit
    (:Is%20Valid
      (CallFunction|BeginTurnServer _unit))
    (:Is%20Not%20Valid
      (CallFunction|EndTurnServer))))

(fn FindAttackTiles
  (params (EnemyUnit :type Unit%20Base%20Object%20Reference) (CurrentMovementTiles :type Array%20of%20Integers))
  (bind _activeunit (Variables|Default|GetActiveUnit))
  ;[1 1 1] Get tiles we can attack "Enemy Unit" from
  (bind _attacktiles_outer (Default|GenerateMovementActors (CallFunction|GetGrid) (Variables|/Game/Blueprints/Grid/GridAnchor.GridAnchor_C|Getindex EnemyUnit) 0 (Variables|/Game/Blueprints/Units/Unit_Base.Unit_Base_C|GetAttackRange _activeunit) (Variables|/Game/Blueprints/Units/Unit_Base.Unit_Base_C|GetMinAttackRange _activeunit) (Utilities|Map|MakeMap "NewEnumerator0" 1.0) true))
  ;[1 1 1] Check if these tiles are within our walkable tiles (can we reach them this turn?)
  (for _array_element _attacktiles_outer
    (if (Utilities|Array|ContainsItem CurrentMovementTiles _array_element)
      (Utilities|Array|AddUnique (LocalVariables|Gettemp%20AttackTiles) _array_element)))
  ;[1 1 1] Return Tiles from which we can attack target, that we can reach this turn
  (return (LocalVariables|Gettemp%20AttackTiles)))