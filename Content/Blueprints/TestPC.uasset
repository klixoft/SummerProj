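; Player controller for a multiplayer turn-based grid tactics game, handling unit selection, destination picking and turn hand-off with TestGM.
; While active, it moves a grid marker under the cursor, and clicks either select a team unit to show range tiles or set a destination and open the Action widget.
; Server events relay choices and movement to the game mode.
; ActiveUnit's OnRep attaches the camera and rebinds the move-finished callback that refreshes range tiles.
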(event Custom|BeginTurn%20Client
  (bind _activeunit (Variables|Default|GetActiveUnit))
  ;[1 1 1] this is where youd wanna add anything like show hud, notify player its his turn etc.
  (Default|GenerateMovementActors (CallFunction|GetGrid) (Variables|/Game/Blueprints/GridANchor.GridAnchor_C|Getindex _activeunit) (Variables|/Game/Blueprints/Unit_Base.Unit_Base_C|GetMovementRange _activeunit) (Variables|/Game/Blueprints/Unit_Base.Unit_Base_C|GetAttackRange _activeunit)))

(event Custom|Unit%20FinishMove
  (CallFunction|ShowRangeTiles (Variables|Default|GetActiveUnit)))

(event Custom|Set%20Destination%20Index%20Server
  (params (Destination :type Integer))
  ;[1 1 1] Ensure your selected destination index is replicated to server
  (bind _output_get (Variables|Default|SetDestinationIndex Destination))
  (Development|PrintString (Utilities|String|ToString(Integer) _output_get)))

(event Custom|Select%20Unit%20Server
  (params (Unit :type Unit%20Base%20Object%20Reference))
  ;[1 1 1] Ensure Active Unit is replicated to Server (and subsequently to relevant player)
  (Variables|Default|SetActiveUnit Unit))

(event Custom|Move%20Unit%20Server
  ;[1 1 1] Ensure Movement is executed on server
  (Default|StartMovement (Variables|Default|GetGameModeRef)))

(event Custom|End%20Turn%20Client
  (Default|ClearMovementActors (CallFunction|GetGrid)))

(event Custom|BeginTurn%20Server
  (params (ActiveUnit :type Unit%20Base%20Object%20Reference))
  ;[1 1 1] Gamemode triggered, notifies this controller of being "active"
  (Variables|Default|SetActiveUnit ActiveUnit)
  (Variables|Default|SetisActive true)
  (CallFunction|BeginTurnClient))

(event Custom|End%20Turn%20Server
  ;[1 1 1] Notify Gamemode of ending turn
  (Variables|Default|SetisActive false)
  (Default|EndPlayerTurn (Variables|Default|GetGameModeRef) self)
  (CallFunction|EndTurnClient)
  (Development|PrintString "End Turn"))

(event EventBeginPlay
  (Variables|Default|SetbShowMouseCursor true)
  (Utilities|FlowControl|Sequence
    (:then_0
      (bind _astest_gm (Utilities|Casting|CastToTestGM (Game|GetGameMode)))
      (Variables|Default|SetGameModeRef _astest_gm))
    (:then_1
      (bind _returnvalue (UserInterface|CreateWidget "/Game/UI/Action.Action_C"))
      (Variables|Default|SetActionWidgetRef _returnvalue))))

(event Input|AxisEvents|InputAxisMouseMove
  (params (AxisValue :type Float%20%28single-precision%29))
  (if (Variables|Default|GetisActive)
    (bind _posindex (CallFunction|SetMarkeronGrid))
    (Default|MoveMarker (CallFunction|GetMarker) _posindex)))

(event Input|MouseEvents|LeftMouseButton
  (params (Key :type Key%20Structure))
  (:Pressed
    (if (Variables|Default|GetisActive)
      (CallFunction|OnClick))))

(fn ConstructionScript)

(fn OnClick
  (bind _hitresult (Game|Player|GetHitResultUnderCursorbyChannel "TraceTypeQuery1" true))
  (bind (_bblockinghit _binitialoverlap _time _distance _location _impactpoint _normal _impactnormal _physmat _hitactor) (Collision|BreakHitResult _hitresult))
  (if _bblockinghit
    (Variables|Default|SetRelativeLocation (- _location (Transformation|GetActorLocation _hitactor)))
    (if (== (Utilities|GetClass _hitactor) "/Game/Blueprints/Unit_Base.Unit_Base_C")
      ;[1 1 1] Team Check for unit selection
      (bind _asunit_base (Utilities|Casting|CastToUnit_Base _hitactor))
      (if (Utilities|Enum|Equal(Enum) (Variables|/Game/Blueprints/Unit_Base.Unit_Base_C|GetTeam _asunit_base) (Variables|Default|GetTeam))
        (CallFunction|SelectUnitServer _asunit_base)
        (CallFunction|ShowRangeTiles _asunit_base)
        (else
          (Development|PrintString "THATS NOT YOUR UNIT!")))
      (elif (== (Utilities|GetClass _hitactor) "/Game/Blueprints/Grid.Grid_C")
        (if (Utilities|Enum|Equal(Enum) (Variables|/Game/Blueprints/Unit_Base.Unit_Base_C|GetTeam (Variables|Default|GetActiveUnit)) (Variables|Default|GetTeam))
          (bind _asgrid (Utilities|Casting|CastToGrid _hitactor))
          (bind _index (Default|VectortoIndex _asgrid (Variables|Default|GetRelativeLocation)))
          (CallFunction|SetDestinationIndexServer _index)
          (UserInterface|Viewport|AddtoViewport (Variables|Default|GetActionWidgetRef) 0)
          (else
            (Development|PrintString "you do not have a player unit selected")))
        (else
          (Development|PrintString "Did not select a grid"))))))

(fn SetMarkeronGrid
  (bind _hmm (Variables|Default|Gethmm))
  (bind (_hitresult _returnvalue) (Class|PlayerController|GetHitResultUnderCursorforObjects _hmm true))
  (bind (_bblockinghit _binitialoverlap _time _distance _location _impactpoint _normal _impactnormal _physmat _hitactor) (Collision|BreakHitResult _hitresult))
  (if _returnvalue
    (Utilities|IsValid (CallFunction|GetGrid)
      (:Is%20Valid
        (Variables|Default|SetRelativeLocation (- _location (Transformation|GetActorLocation _hitactor)))
        (bind _index (Default|VectortoIndex (CallFunction|GetGrid) (Variables|Default|GetRelativeLocation)))
        (return _index)))))

(fn GetMarker
  (Utilities|IsValid (Variables|Default|GetMarker)
    (:Is%20Valid
      _)
    (:Is%20Not%20Valid
      (bind _returnvalue (Game|SpawnActorfromClass "/Game/Blueprints/MarkerBP.MarkerBP_C" (Math|Transform|MakeTransform "0, 0, 0" "0, 0, 0" "1,1,1") "Undefined" 0 0))
      (bind _output_get (Variables|Default|SetMarker _returnvalue))))
  (return _output_get))

(fn OnRepActiveUnit
  (bind _returnvalue (Pawn|GetControlledPawn))
  (bind _activeunit (Variables|Default|GetActiveUnit))
  ;[1 1 1] this is when we receive "replicated" value for Active Unit, ensure camera goes to it
  (Utilities|FlowControl|Sequence
    (:then_0
      (Utilities|IsValid (Variables|Default|GetOld_ActiveUnit)
        (:Is%20Valid
          (EventDispatchers|UnbindallEventsfromMoveFinished (Variables|Default|GetOld_ActiveUnit)))))
    (:then_1
      (Variables|Default|SetOld_ActiveUnit _activeunit)
      (Utilities|IsValid _activeunit
        (:Is%20Valid
          (EventDispatchers|BindEventtoMoveFinished _activeunit (EventDispatchers|CreateEvent :!event Custom|Unit%20FinishMove))
          (if (.bSuccess (Utilities|Casting|CastToDefaultCamera (Pawn|GetControlledPawn)))
            (Transformation|AttachActorToActor _returnvalue _activeunit "None" "SnapToTarget" "KeepWorld" "SnapToTarget" true)
            (Transformation|SetActorRelativeTransform _returnvalue (Math|Transform|MakeTransform "0, 0,800.000000" "-90.000000, 0, 0" "1,1,1") false false)))
        (:Is%20Not%20Valid
          (Default|ClearMovementActors (CallFunction|GetGrid)))))))

(fn GetGrid
  (Utilities|IsValid (Variables|Default|GetGridRef)
    (:Is%20Valid
      (return (Variables|Default|GetGridRef)))
    (:Is%20Not%20Valid
      (bind _outactors (Actor|GetAllActorsOfClass "/Game/Blueprints/Grid.Grid_C"))
      (if (Utilities|Array|IsValidIndex _outactors)
        (bind _output_get (Variables|Default|SetGridRef (Utilities|Array|Get(acopy) _outactors)))
        (return _output_get)
        (else
          (return 0))))))

(fn ShowRangeTiles
  (params (Unit :type Unit%20Base%20Object%20Reference))
  (Default|GenerateMovementActors (CallFunction|GetGrid) (Variables|/Game/Blueprints/GridANchor.GridAnchor_C|Getindex Unit) (select (Variables|/Game/Blueprints/Unit_Base.Unit_Base_C|GetMovedThisTurn? Unit) 0 (Variables|/Game/Blueprints/Unit_Base.Unit_Base_C|GetMovementRange Unit)) (Math|Float|SelectFloat 0.0 (Variables|/Game/Blueprints/Unit_Base.Unit_Base_C|GetAttackRange Unit) (Variables|/Game/Blueprints/Unit_Base.Unit_Base_C|GetActedThisTurn? Unit))))