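; GridAnchor is an actor that snaps its static mesh to a tile on a Grid actor while the anchor itself stays freely placed.
; The construction script finds the first Grid if none is referenced, attaches to it, then runs GridSnapping; there is no runtime logic.
; GridSnapping converts relative location to a tile Index and moves the mesh there, or sets -1 and returns it to the actor when a new index is invalid.
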(event EventBeginPlay)

(event EventTick
  (params (DeltaSeconds :type Float%20%28single-precision%29)))

(fn ConstructionScript
  (Utilities|IsValid (Variables|Default|GetGridRef)
    (:Is%20Valid
      _)
    (:Is%20Not%20Valid
      (bind _outactors (Actor|GetAllActorsOfClass "/Game/Blueprints/Grid/Grid.Grid_C"))
      (bind _output_get (Variables|Default|SetGridRef (Utilities|Array|Get(acopy) _outactors)))
      (Transformation|AttachActorToActor _output_get "None" "KeepRelative" "KeepRelative" "KeepRelative" true)))
  (Utilities|IsValid (Variables|Default|GetGridRef)
    (:Is%20Valid
      (CallFunction|GridSnapping))))

(fn GridSnapping
  (bind _gridref (Variables|Default|GetGridRef))
  (bind _defaultsceneroot (Variables|Default|GetDefaultSceneRoot))
  (bind _relativelocation (Variables|/Script/Engine.SceneComponent|GetRelativeLocation _defaultsceneroot))
  (bind _index (Default|VectortoIndex _gridref _relativelocation))
  (if (!= (Variables|Default|Getindex) _index)
    (if (Utilities|Array|IsValidIndex (Variables|/Game/Blueprints/Grid/Grid.Grid_C|GetGridArray (Variables|Default|GetGridRef)) _index)
      _
      (else
        ;[1 1 1] snap mesh to actor anchor if outside of grid
        (Variables|Default|Setindex -1)
        (Transformation|SetWorldLocation (Variables|Default|GetStaticMesh) (Transformation|GetActorLocation) false true)
        (return))))
  ;[1 1 1] if index changed, update position of mesh
  (bind _output_get (Variables|Default|Setindex _index))
  (Transformation|SetWorldLocation (Variables|Default|GetStaticMesh) (Default|IndextoLocation (Variables|Default|GetGridRef) _output_get true) false true)
  (return))