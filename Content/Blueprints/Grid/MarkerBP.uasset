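; MarkerBP is a marker actor that shows a position on the grid by snapping its static mesh to a cell.
; Its MoveMarker event takes a cell index, checks it against the GridRef's GridArray, and sets the mesh's world location to that cell's CellLocation.
; Invalid indices are ignored, and the mesh moves without sweep or teleport.
; BeginPlay, overlap and Tick are unused.
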(event Custom|MoveMarker
  (params (LocalIndex :type Integer))
  (bind _gridref (Variables|Default|GetGridRef))
  (bind _gridarray (Variables|/Game/Blueprints/Grid/Grid.Grid_C|GetGridArray _gridref))
  (if (Utilities|Array|IsValidIndex _gridarray LocalIndex)
    (Transformation|SetWorldLocation (Variables|Default|GetStaticMesh) (.CellLocation (Utilities|Struct|BreakS_CellData (Utilities|Array|Get(acopy) _gridarray LocalIndex))) false false)))

(event EventBeginPlay
  (|CallParentFunction) ; This node is disabled and will not be called.\nDrag off pins to build functionality.
)

(event Collision|EventActorBeginOverlap
  (params (OtherActor :type Actor%20Object%20Reference))
  (|CallParentFunction OtherActor) ; This node is disabled and will not be called.\nDrag off pins to build functionality.
)

(event EventTick
  (params (DeltaSeconds :type Float%20%28single-precision%29))
  (|CallParentFunction DeltaSeconds) ; This node is disabled and will not be called.\nDrag off pins to build functionality.
)

(fn ConstructionScript
  (|CallParentFunction))