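; GridAnchor is an actor that occupies an indexed position on a Grid actor and can be moved to another index.
; Its construction script takes the first Grid found when GridRef is unset, attaches to it, then stores the index returned by GridSnappingCube.
; OnClickMove teleport-free sets the actor to the given index's location, zeroes the mesh's relative location and updates the stored index.
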(event EventBeginPlay)

(event Collision|EventActorBeginOverlap
  (params (OtherActor :type Actor%20Object%20Reference)))

(event EventTick
  (params (DeltaSeconds :type Float%20%28single-precision%29)))

(fn ConstructionScript
  (Utilities|IsValid (Variables|Default|GetGridRef)
    (:Is%20Valid
      _)
    (:Is%20Not%20Valid
      (bind _outactors (Actor|GetAllActorsOfClass "/Game/Blueprints/Grid.Grid_C"))
      (bind _output_get (Variables|Default|SetGridRef (Utilities|Array|Get(acopy) _outactors)))
      (Transformation|AttachActorToActor _output_get "None" "KeepRelative" "KeepRelative" "KeepRelative" true)))
  (Utilities|IsValid (Variables|Default|GetGridRef)
    (:Is%20Valid
      (bind _index (Default|GridSnappingCube (Variables|Default|GetGridRef) self))
      (Variables|Default|Setindex _index))))

(fn OnClickMove
  (params (localIndex :type Integer))
  (Transformation|SetActorLocation (Default|IndextoLocation (Variables|Default|GetGridRef) localIndex) false false)
  (Transformation|SetRelativeLocation (Variables|Default|GetStaticMesh) "0, 0, 0" false false)
  (Variables|Default|Setindex localIndex))