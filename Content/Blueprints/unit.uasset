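; Grid-based unit actor that snaps to tiles when placed and can interact with overlapping actors.
; The construction script attaches it to the first Grid found, derives a tile index from relative location and snaps only the mesh, falling back to the actor anchor when out of range.
; BeginPlay moves the actor to the saved snap position and re-centres the mesh.
; Interact input or the pop event sends InteractMessage to the first overlapping Interact_Interface implementer.
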(event Custom|pop
  (Development|PrintString "Hello")
  (bind _array_element (Utilities|Array|ForEachLoopwithBreak (Collision|GetOverlappingActors "/Script/Engine.Actor" :!class /Script/Engine.Actor) :!label _label)
    (:LoopBody
      (if (Utilities|DoesObjectImplementInterface _array_element "/Game/Inventory/Interact_Interface.Interact_Interface_C")
        (Class|InteractInterface|Interact(Message) _array_element)
        (goto _label Break)))))

(event EventBeginPlay
  (Transformation|SetActorLocation (Variables|Default|GetTempCurrentSnap) false true)
  (Transformation|SetRelativeLocation (Variables|Default|GetStaticMesh) "0, 0, 0" false true))

(event Collision|EventActorBeginOverlap
  (params (OtherActor :type Actor%20Object%20Reference)))

(event EventTick
  (params (DeltaSeconds :type Float%20%28single-precision%29)))

(event Input|ActionEvents|InputActionInteract
  (params (Key :type Key%20Structure))
  (:Pressed
    (Development|PrintString "Hello")
    (bind _array_element (Utilities|Array|ForEachLoopwithBreak (Collision|GetOverlappingActors "/Script/Engine.Actor" :!class /Script/Engine.Actor) :!label _label)
      (:LoopBody
        (if (Utilities|DoesObjectImplementInterface _array_element "/Game/Inventory/Interact_Interface.Interact_Interface_C")
          (Class|InteractInterface|Interact(Message) _array_element)
          (goto _label Break))))))

(fn ConstructionScript
  (Development|PrintString (Utilities|String|ToString(Vector) (Transformation|GetActorLocation)))
  (Utilities|IsValid (Variables|Default|GetGridRef)
    (:Is%20Valid
      _)
    (:Is%20Not%20Valid
      (bind _outactors (Actor|GetAllActorsOfClass "/Game/Blueprints/Grid.Grid_C"))
      (bind _output_get (Variables|Default|SetGridRef (Utilities|Array|Get(acopy) _outactors)))
      (Transformation|AttachActorToActor _output_get "None" "KeepRelative" "KeepRelative" "KeepRelative" true)))
  (Utilities|IsValid (Variables|Default|GetGridRef)
    (:Is%20Valid
      (if (!= (Variables|Default|Getindex) (+ (* (Math|Float|Round (.x (/ (Variables|/Script/Engine.SceneComponent|GetRelativeLocation (Variables|Default|GetDefaultSceneRoot)) (Variables|/Game/Blueprints/Grid.Grid_C|GetTileSize (Variables|Default|GetGridRef))))) (Variables|/Game/Blueprints/Grid.Grid_C|GetMaxX (Variables|Default|GetGridRef))) (Math|Float|Round (.y (/ (Variables|/Script/Engine.SceneComponent|GetRelativeLocation (Variables|Default|GetDefaultSceneRoot)) (Variables|/Game/Blueprints/Grid.Grid_C|GetTileSize (Variables|Default|GetGridRef)))))))
        (if (Math|Boolean|ANDBoolean (Math|Integer|InRange(Integer) (Math|Float|Round (.x (/ (Variables|/Script/Engine.SceneComponent|GetRelativeLocation (Variables|Default|GetDefaultSceneRoot)) (Variables|/Game/Blueprints/Grid.Grid_C|GetTileSize (Variables|Default|GetGridRef))))) 0 (Variables|/Game/Blueprints/Grid.Grid_C|GetMaxX (Variables|Default|GetGridRef)) true false) (Math|Integer|InRange(Integer) (Math|Float|Round (.y (/ (Variables|/Script/Engine.SceneComponent|GetRelativeLocation (Variables|Default|GetDefaultSceneRoot)) (Variables|/Game/Blueprints/Grid.Grid_C|GetTileSize (Variables|Default|GetGridRef))))) 0 (Variables|/Game/Blueprints/Grid.Grid_C|GetMaxY (Variables|Default|GetGridRef)) true false) (Utilities|Array|IsValidIndex (Variables|/Game/Blueprints/Grid.Grid_C|GetGridPositions (Variables|Default|GetGridRef)) (+ (* (Math|Float|Round (.x (/ (Variables|/Script/Engine.SceneComponent|GetRelativeLocation (Variables|Default|GetDefaultSceneRoot)) (Variables|/Game/Blueprints/Grid.Grid_C|GetTileSize (Variables|Default|GetGridRef))))) (Variables|/Game/Blueprints/Grid.Grid_C|GetMaxX (Variables|Default|GetGridRef))) (Math|Float|Round (.y (/ (Variables|/Script/Engine.SceneComponent|GetRelativeLocation (Variables|Default|GetDefaultSceneRoot)) (Variables|/Game/Blueprints/Grid.Grid_C|GetTileSize (Variables|Default|GetGridRef))))))))
          ;[1 1 1] if index changed, update position of mesh
          (bind _output_get_2 (Variables|Default|Setindex (+ (* (Math|Float|Round (.x (/ (Variables|/Script/Engine.SceneComponent|GetRelativeLocation (Variables|Default|GetDefaultSceneRoot)) (Variables|/Game/Blueprints/Grid.Grid_C|GetTileSize (Variables|Default|GetGridRef))))) (Variables|/Game/Blueprints/Grid.Grid_C|GetMaxX (Variables|Default|GetGridRef))) (Math|Float|Round (.y (/ (Variables|/Script/Engine.SceneComponent|GetRelativeLocation (Variables|Default|GetDefaultSceneRoot)) (Variables|/Game/Blueprints/Grid.Grid_C|GetTileSize (Variables|Default|GetGridRef))))))))
          (Variables|Default|SetTempCurrentSnap (Utilities|Array|Get(acopy) (Variables|/Game/Blueprints/Grid.Grid_C|GetGridPositions (Variables|Default|GetGridRef)) _output_get_2))
          (Transformation|SetWorldLocation (Variables|Default|GetStaticMesh) (Variables|Default|GetTempCurrentSnap) false true)
          (else
            ;[1 1 1] snap mesh to actor anchor if outside of grid
            (Variables|Default|Setindex -1)
            (Transformation|SetWorldLocation (Variables|Default|GetStaticMesh) (Transformation|GetActorLocation) false true)))
        (else
          ;[1 1 1] ensure mesh snapped to grid when moving actor anchor
          (Transformation|SetWorldLocation (Variables|Default|GetStaticMesh) (Variables|Default|GetTempCurrentSnap) false true))))))