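; Base actor for a grid unit in a turn-based game, handling its movement along a tile path.
; BeginPlay moves the actor to its mesh's world location and zeroes the mesh offset.
; Move_Unit uses the MoveSmoothly macro, a manually continued reverse loop, so each latent MoveComponentTo finishes before the next tile.
; On completion it sets Index to the path's first element, flags MovedThisTurn and calls MoveFinished.
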(event Custom|Move_Unit
  (params (Path :type Array%20of%20Integers))
  (bind _nextpoint (Utilities|MoveSmoothly Path :!label _label)
    (:Move
      (Transformation|SetRelativeLocation (Variables|Default|GetStaticMesh) "0, 0, 0" false false)
      (Components|MoveComponentTo (Variables|Default|GetDefaultSceneRoot) (Default|IndextoLocation (Variables|Default|GetGridRef) _nextpoint true) "0, 0, 0" false false 0.5 false)
      (goto _label Continue))
    (:Completed
      (Variables|Default|Setindex (Utilities|Array|Get(acopy) Path))
      (Variables|Default|SetMovedThisTurn? true)
      (Default|CallMoveFinished))))

(event EventBeginPlay
  (|CallParentFunction)
  (Transformation|SetActorLocation (Transformation|GetWorldLocation (Variables|Default|GetStaticMesh)) false true)
  (Transformation|SetRelativeLocation (Variables|Default|GetStaticMesh) "0, 0, 0" false true))

(event Collision|EventActorBeginOverlap
  (params (OtherActor :type Actor%20Object%20Reference))
  (|CallParentFunction OtherActor) ; This node is disabled and will not be called.\nDrag off pins to build functionality.
)

(event EventTick
  (params (DeltaSeconds :type Float%20%28single-precision%29))
  (|CallParentFunction DeltaSeconds) ; This node is disabled and will not be called.\nDrag off pins to build functionality.
)

(fn ConstructionScript
  (|CallParentFunction))