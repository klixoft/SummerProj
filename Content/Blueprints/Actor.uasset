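; Base actor meant to snap onto a Grid actor in the level, with the snapping logic still an empty stub.
; On BeginPlay it caches the Grid reference if exactly one exists, otherwise printing a "Too Many Grids Present" message, even when none exists.
; SnapToLocation is called after that check and from the construction script, where the grid lookup does not run.
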(event EventBeginPlay
  (CallFunction|GridCheck)
  (CallFunction|SnaptoLocation))

(event Collision|EventActorBeginOverlap
  (params (OtherActor :type Actor%20Object%20Reference)))

(event EventTick
  (params (DeltaSeconds :type Float%20%28single-precision%29)))

(fn ConstructionScript
  (CallFunction|SnaptoLocation))

(fn SnaptoLocation)

(fn GridCheck
  (bind _outactors (Actor|GetAllActorsOfClass "/Game/Blueprints/Grid.Grid_C"))
  (if (== (Utilities|Array|Length _outactors) 1)
    (Variables|Default|SetGridRef (Utilities|Array|Get(acopy) _outactors))
    (else
      (Development|PrintString "Too Many Grids Present"))))