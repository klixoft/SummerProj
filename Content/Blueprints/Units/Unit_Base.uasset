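; Base grid unit for a turn-based tactics game, with stats, path movement and health.
; The construction script loads stats from a data table by class and rank.
; Move_Unit uses a resumable MoveSmoothly loop to step through the path from last element to first, turning and interpolating between tiles, then flags the unit as moved.
; AnyDamage subtracts formula-adjusted damage, at least 1, and destroys the unit at zero health.
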(event Custom|Move_Unit
  (params (Path :type Array%20of%20Integers))
  (bind _nextpoint (Utilities|MoveSmoothly Path :!label _label)
    (:Move
      (Transformation|SetRelativeLocation (Variables|Default|GetSkeletalMesh) "0, 0, 0" false false)
      (Components|MoveComponentTo (Variables|Default|GetDefaultSceneRoot) (Default|IndextoLocation (Variables|Default|GetGridRef) _nextpoint true) (Math|Rotator|MakeRotator 0.0 0.0 (.yaw (Math|Rotator|FindLookatRotation (Transformation|GetActorLocation) (Default|IndextoLocation (Variables|Default|GetGridRef) _nextpoint true)))) false false 0.5 true)
      (goto _label Continue))
    (:Completed
      (Variables|Default|Setindex (Utilities|Array|Get(acopy) Path))
      (Variables|Default|SetMovedThisTurn? true)
      (Default|CallMoveFinished))))

(event EventBeginPlay
  (|CallParentFunction)
  (Transformation|SetActorLocation (Transformation|GetWorldLocation (Variables|Default|GetSkeletalMesh)) false true)
  (Transformation|SetRelativeLocation (Variables|Default|GetSkeletalMesh) "0, 0, 0" false false))

(event Collision|EventActorBeginOverlap
  (params (OtherActor :type Actor%20Object%20Reference))
  (|CallParentFunction OtherActor) ; This node is disabled and will not be called.\nDrag off pins to build functionality.
)

(event EventTick
  (params (DeltaSeconds :type Float%20%28single-precision%29))
  (|CallParentFunction DeltaSeconds) ; This node is disabled and will not be called.\nDrag off pins to build functionality.
)

(event Game|Damage|EventAnyDamage
  (params (Damage :type Float%20%28single-precision%29) (DamageType :type Damage%20Type%20Object%20Reference) (InstigatedBy :type Controller%20Object%20Reference) (DamageCauser :type Actor%20Object%20Reference))
  (bind _output_get (Variables|Default|SetHealth (- (stale _output_get) (Math|Integer|Max(Integer) (Math|Float|Truncate (|(Damage*(1-({59A4446E-4565-CFBF-C1CF-C585BF22949B}/(Damage*2)))) Damage)) 1))))
  (if (<= _output_get 0)
    (Actor|DestroyActor)))

(fn ConstructionScript
  (bind _class (Variables|Default|GetClass))
  (bind (_class_2 _rank) (Utilities|Struct|BreakUnit_Class_Rank_BP _class))
  (|CallParentFunction)
  (CallFunction|UpdateStats _class_2 _rank))

(fn CalculateDamage
  (params (Damage :type Float%20%28single-precision%29)))

(fn UpdateStats
  (params (Class :type Unit_Classes%20Enum :default "NewEnumerator0") (Rank :type Rank%20Enum :default "NewEnumerator0"))
  (bind _returnvalue (Utilities|GetDataTableRow "/Game/Blueprints/Units/Unit_Data_Table.Unit_Data_Table" (Utilities|String|StringToName (Utilities|String|EnumtoString Class)))
    (:then
      (bind _output_get (Variables|Default|SetHealth (.Health (Utilities|Struct|BreakStats (Utilities|Array|Get(acopy) (.Rank (Utilities|Struct|BreakUnit_Data_Struct _returnvalue)) (Math|Conversions|ToInteger(Byte) Rank))))))
      (Variables|Default|SetMaxHealth _output_get)
      (Variables|Default|SetAttack (.Attack (Utilities|Struct|BreakStats (Utilities|Array|Get(acopy) (.Rank (Utilities|Struct|BreakUnit_Data_Struct _returnvalue)) (Math|Conversions|ToInteger(Byte) Rank)))))
      (Variables|Default|SetDefence (.defence (Utilities|Struct|BreakStats (Utilities|Array|Get(acopy) (.Rank (Utilities|Struct|BreakUnit_Data_Struct _returnvalue)) (Math|Conversions|ToInteger(Byte) Rank)))))
      (Variables|Default|SetMovementRange (.Movement (Utilities|Struct|BreakStats (Utilities|Array|Get(acopy) (.Rank (Utilities|Struct|BreakUnit_Data_Struct _returnvalue)) (Math|Conversions|ToInteger(Byte) Rank)))))
      (Variables|Default|SetMinAttackRange (.MinimumRange (Utilities|Struct|BreakStats (Utilities|Array|Get(acopy) (.Rank (Utilities|Struct|BreakUnit_Data_Struct _returnvalue)) (Math|Conversions|ToInteger(Byte) Rank)))))
      (Variables|Default|SetAttackRange (.MaxRange (Utilities|Struct|BreakStats (Utilities|Array|Get(acopy) (.Rank (Utilities|Struct|BreakUnit_Data_Struct _returnvalue)) (Math|Conversions|ToInteger(Byte) Rank))))))))