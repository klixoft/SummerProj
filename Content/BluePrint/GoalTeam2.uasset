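; Team goal that detects the gravity ball entering its score box and colors its mesh by owning team.
; On the server, a DoOnce with a timed reset debounces overlaps, respawns the ball through BallSpawner and has UberBall_GameMode credit the opposing team.
; The ball's last player earns personal points in GameplayPS, and the assisting player earns fewer if the pass was recent.
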(event OnComponentBeginOverlap(Score_Box)
  (params (OverlappedComponent :type Primitive%20Component%20Object%20Reference) (OtherActor :type Actor%20Object%20Reference) (OtherComp :type Primitive%20Component%20Object%20Reference) (OtherBodyIndex :type Integer) (bFromSweep :type Boolean) (SweepResult :type Hit%20Result%20Structure%20%28by%20ref%29))
  (Networking|SwitchHasAuthority
    (:Authority
      (bind _asbp_gravity_ball (Utilities|Casting|CastToBP_GravityBall OtherActor))
      (Utilities|FlowControl|DoOnce false :!label _label
        (:Completed
          (Utilities|FlowControl|Sequence
            (:then_0
              (Utilities|FlowControl|Delay 2.0)
              (goto _label Reset))
            (:then_1
              (bind _outactors (Actor|GetAllActorsOfClass "/Game/BluePrint/BallSpawner.BallSpawner_C"))
              (Utilities|IsValid (Utilities|Array|Get(acopy) _outactors)
                (:Is%20Valid
                  (Default|RespawnBall (Utilities|Array|Get(acopy) _outactors)))))
            (:then_2
              (Networking|SwitchHasAuthority
                (:Authority
                  (bind _asuber_ball_game_mode (Utilities|Casting|CastToUberBall_GameMode (Game|GetGameMode)))
                  (Default|AddScore _asuber_ball_game_mode (Utilities|Select :Index (Variables|Default|GetTeam) :NewEnumerator2 "NewEnumerator2" :NewEnumerator0 (Utilities|Enum|LiteralenumTeamEnums "NewEnumerator1") :NewEnumerator1 (Utilities|Enum|LiteralenumTeamEnums "NewEnumerator0"))))))
            (:then_3
              ;[1 1 1] deals with calculating possible assists
              (if (Math|Float|NearlyEqual(Float) (Utilities|Time|GetGameTimeinSeconds) (Variables|/Game/BluePrint/BP_GravityBall.BP_GravityBall_C|GetAssist_Pass_Time _asbp_gravity_ball) 5.0)
                (if (and (Utilities|IsValid (Variables|/Game/BluePrint/BP_GravityBall.BP_GravityBall_C|GetAssistingPlayer _asbp_gravity_ball)) (Utilities|IsValid (Variables|/Game/BluePrint/BP_GravityBall.BP_GravityBall_C|GetLastPlayer _asbp_gravity_ball)))
                  (Utilities|FlowControl|Sequence
                    (:then_0
                      (bind _asgameplay_ps (Utilities|Casting|CastToGameplayPS (Variables|/Script/Engine.Pawn|GetPlayerState (Variables|/Game/BluePrint/BP_GravityBall.BP_GravityBall_C|GetAssistingPlayer _asbp_gravity_ball))))
                      (bind _output_get (Variables|/Game/BluePrint/GameplayPS.GameplayPS_C|SetPoint _asgameplay_ps (+ (stale _output_get) 1))))
                    (:then_1
                      (bind _asgameplay_ps_2 (Utilities|Casting|CastToGameplayPS (Variables|/Script/Engine.Pawn|GetPlayerState (Variables|/Game/BluePrint/BP_GravityBall.BP_GravityBall_C|GetLastPlayer _asbp_gravity_ball)) :!label _label_2))
                      (bind _output_get_2 (Variables|/Game/BluePrint/GameplayPS.GameplayPS_C|SetPoint _asgameplay_ps_2 (+ (stale _output_get_2) 3)))))
                  (else
                    (goto _label_2)))
                (else
                  (goto _label_2))))))))))

(fn ConstructionScript
  (Rendering|Material|SetMaterial (Variables|Default|GetStaticMesh) 0 (Utilities|Select :Index (Variables|Default|GetTeam) :NewEnumerator2 0 :NewEnumerator0 "/Game/BluePrint/TeamOneColor.TeamOneColor" :NewEnumerator1 "/Game/BluePrint/TeamTwoColor.TeamTwoColor")))