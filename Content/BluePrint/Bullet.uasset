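; Bullet actor that damages what it overlaps and then destroys itself, with a fixed lifespan set on BeginPlay as a fallback.
; Overlaps route into TargetHit, which ignores the Instigator and applies Damage credited to the instigator's controller, with the Owner as damage causer.
; Damage is skipped when the Owner is invalid, but the bullet is still destroyed.
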(event EventBeginPlay
  (Actor|SetLifeSpan 2e+01))

(event EventActorBeginOverlap
  (params (OtherActor :type Actor%20Object%20Reference))
  (CallFunction|TargetHit OtherActor))

(fn ConstructionScript)

(fn TargetHit
  (params (InHitActor :type Actor%20Object%20Reference))
  (bind _returnvalue (Components|GetOwner))
  (LocalVariables|SetLHitActor InHitActor)
  (if (!= InHitActor (Variables|Actor|GetInstigator))
    (Utilities|IsValid _returnvalue
      (:Is%20Valid
        (Game|Damage|ApplyDamage (LocalVariables|GetLHitActor) (Variables|Default|GetDamage) (Game|GetInstigatorController) _returnvalue))
      (:Is%20Not%20Valid
        _))
    (Actor|DestroyActor)))